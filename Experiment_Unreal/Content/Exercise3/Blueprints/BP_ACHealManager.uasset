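; BP_ACHealManager is a health manager, apparently an actor component, that stores and updates a current health value.
; Init sets current health from InitLife, and SetDamage subtracts damage, clamping the result between zero and MaxHealth.
; GetPercentage returns current health as a fraction of MaxHealth.
; The event graph has no active logic, so health changes only when these functions are called.
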(fn `Get Percentage`
  (returns (percentage :type "Float (double-precision)"))
  (return (/ (`self.CurrentHealth`) (`self.MaxHealth`))))

(fn `Init`
  (set `self.CurrentHealth` (`self.InitLife`)))

(fn `SetDamage`
  (params (Damage :type "Float (double-precision)"))
  (set `self.CurrentHealth` (`KismetMathLibrary.FClamp` (- (`self.CurrentHealth`) Damage) 0.0 (`self.MaxHealth`))))