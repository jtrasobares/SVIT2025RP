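; BP_Exercise1HUD is the HUD Blueprint that owns the inventory widget for Exercise 1.
; On BeginPlay it creates a BP_WBInventory widget for player controller 0, stores the reference and adds it to the viewport.
; Its UpdateInventory, SetItemInfo and ClearInfo functions forward to that widget to refresh the inventory and set or clear item info, acting as a thin pass-through.
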(event `self.ReceiveBeginPlay`
  (bind _returnvalue (`|CreateWidget` "/Game/Exercise1/Blueprints/BP_WBInventory.BP_WBInventory_C" (`GameplayStatics.GetPlayerController` 0)))
  (set `self.InventoryRef` _returnvalue)
  (`UserWidget.AddToViewport` _returnvalue 0))

(fn `ClearInfo`
  (`/Game/Exercise1/Blueprints/BP_WBInventory.ClearInfoItem` (`self.InventoryRef`)))

(fn `SetItemInfo`
  (params (ItemInfo :type "/Game/Exercise1/Blueprints/BP_SItem Structure"))
  (`/Game/Exercise1/Blueprints/BP_WBInventory.SetInfoItem` (`self.InventoryRef`) ItemInfo))

(fn `UpdateInventory`
  (`/Game/Exercise1/Blueprints/BP_WBInventory.UpdateInventory` (`self.InventoryRef`)))

(fn `UserConstructionScript`)