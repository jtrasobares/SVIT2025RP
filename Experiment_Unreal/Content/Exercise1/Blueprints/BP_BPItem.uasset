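; Pickup item actor that adds itself to the player's inventory when walked into.
; Its Box overlap event accepts only player character 0 and looks up that character's BP_ACInventory component.
; It passes its IDItem to AddItem and, only if that succeeds, calls PaintWidget on the inventory and destroys itself.
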(event `self.Box.OnComponentBeginOverlap`
  (params (OverlappedComponent :type "PrimitiveComponent Object Reference") (OtherActor :type "Actor Object Reference") (OtherComp :type "PrimitiveComponent Object Reference") (OtherBodyIndex :type Integer) (bFromSweep :type Boolean) (SweepResult :type "HitResult Structure (by ref)"))
  (bind _returnvalue (`self.GetComponentByClass` (`GameplayStatics.GetPlayerCharacter` 0) "/Game/Exercise1/Blueprints/BP_ACInventory.BP_ACInventory_C"))
  (if (== OtherActor (`GameplayStatics.GetPlayerCharacter` 0))
    (`/Engine/EditorBlueprintResources/StandardMacros.IsValid` _returnvalue
      (:`Is Valid`
        (bind _success (`/Game/Exercise1/Blueprints/BP_ACInventory.AddItem` _returnvalue (`self.IDItem`)))
        (if _success
          (`/Game/Exercise1/Blueprints/BP_ACInventory.PaintWidget` _returnvalue)
          (`self.K2_DestroyActor`))))))

(fn `UserConstructionScript`)