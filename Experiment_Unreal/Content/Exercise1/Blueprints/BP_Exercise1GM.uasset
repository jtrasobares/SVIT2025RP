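; Game mode for Exercise 1 that gives the player character an inventory filled with every item in the BP_DTItems data table.
; On BeginPlay it waits one tick, adds a BP_ACInventory component, adds each table row name as an item, then has BP_Exercise1HUD update its inventory.
; An unfinished, disconnected TO DO chain for setting item info on the HUD with a delayed index never runs.
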(event `self.ReceiveBeginPlay`
  (`KismetSystemLibrary.DelayUntilNextTick`)
  (bind _returnvalue (`|AddComponentByClass` (`GameplayStatics.GetPlayerCharacter` 0) "/Game/Exercise1/Blueprints/BP_ACInventory.BP_ACInventory_C"))
  (bind _outrownames (`DataTableFunctionLibrary.GetDataTableRowNames` "/Game/Exercise1/Blueprints/BP_DTItems.BP_DTItems"))
  (set `self.Out Row Names` _outrownames)
  (for _array_element _outrownames
    (`/Game/Exercise1/Blueprints/BP_ACInventory.AddItem` _returnvalue _array_element))
  (bind _asbp_exercise_1hud (cast `/Game/Exercise1/Blueprints/BP_Exercise1HUD` (`PlayerController.GetHUD` (`GameplayStatics.GetPlayerController` 0))))
  (set `self.HUDTest3Ref` _asbp_exercise_1hud)
  (`/Game/Exercise1/Blueprints/BP_Exercise1HUD.UpdateInventory` _asbp_exercise_1hud)
  (if (< (`self.IndexName`) (- (`KismetArrayLibrary.Array_Length` (`self.Out Row Names`)) 1))
    _))

(fn `UserConstructionScript`)