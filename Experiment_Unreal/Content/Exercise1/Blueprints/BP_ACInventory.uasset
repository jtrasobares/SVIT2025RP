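; Inventory component that stores a player's items in a map keyed by item ID, holding one of each with no quantities.
; AddItem copies the row from the BP_DTItems data table, rejecting unknown or already held IDs.
; FindITem and DeleteItem look up and remove entries by ID.
; PaintWidget separately asks player 0's BP_Exercise1HUD to update the inventory display, as item changes do not trigger it here.
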(fn `AddItem`
  (params (IDItem :type Name))
  (returns (success :type Boolean))
  (bind _itemsmap (`self.ItemsMap`))
  (bind _returnvalue (`|GetDataTableRow` "/Game/Exercise1/Blueprints/BP_DTItems.BP_DTItems" IDItem)
    (:`then`
      ;[1 1 1] Unique item not quantity
      (if (`.ReturnValue` (`BlueprintMapLibrary.Map_Find` _itemsmap IDItem))
        (return false)
        (else
          (`BlueprintMapLibrary.Map_Add` _itemsmap IDItem _returnvalue)
          (return true))))
    (:`RowNotFound`
      (return false))))

(fn `DeleteItem`
  (params (ItemID :type Name))
  (returns (IsRemove :type Boolean))
  (bind _returnvalue (`BlueprintMapLibrary.Map_Remove` (`self.ItemsMap`) ItemID))
  (return _returnvalue))

(fn `FindITem`
  (params (ItemID :type Name))
  (returns (isFind :type Boolean) (Item :type "/Game/Exercise1/Blueprints/BP_SItem Structure"))
  (bind (_value _returnvalue) (`BlueprintMapLibrary.Map_Find` (`self.ItemsMap`) ItemID))
  (if _returnvalue
    (return true _value)
    (else
      (return false))))

(fn `PaintWidget`
  (bind _ashud_test_3 (cast `/Game/Exercise1/Blueprints/BP_Exercise1HUD` (`PlayerController.GetHUD` (`GameplayStatics.GetPlayerController` 0))))
  (`/Game/Exercise1/Blueprints/BP_Exercise1HUD.UpdateInventory` _ashud_test_3))